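; BP_Grenade is a thrown grenade actor that explodes after a fuse triggered by its first impact.
; On BeginPlay its Sphere simulates physics and is launched by a velocity-change impulse from ThrowVelocity.
; The first hit, gated by DoOnce, raises damping, prints a debug string and places a temporary decal.
; After a delay it spawns explosion effects and sound, applies radial damage and destroys itself.
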(event `self.ReceiveBeginPlay`
  (`PrimitiveComponent.SetSimulatePhysics` (`self.Sphere`) true)
  (`PrimitiveComponent.AddImpulse` (`self.Sphere`) (`self.ThrowVelocity`) "None" true))

(event `self.Sphere.OnComponentHit`
  (params (HitComponent :type "PrimitiveComponent Object Reference") (OtherActor :type "Actor Object Reference") (OtherComp :type "PrimitiveComponent Object Reference") (NormalImpulse :type "Vector Structure") (Hit :type "HitResult Structure (by ref)"))
  (bind _returnvalue (`self.K2_GetActorLocation`))
  (`/Engine/EditorBlueprintResources/StandardMacros.DoOnce` false
    (:`Completed`
      (`PrimitiveComponent.SetLinearDamping` (`self.Sphere`) 5.0)
      (`KismetSystemLibrary.PrintString` "Hello")
      (`GameplayStatics.SpawnDecalAtLocation` "/Game/Materials/GrenadeDecal.GrenadeDecal" (300.0 300.0 300.0) (`self.K2_GetActorLocation`) (struct :`Pitch` -90.0) 2.7)
      (`KismetSystemLibrary.Delay` 3.0)
      (`GameplayStatics.SpawnEmitterAtLocation` "/Game/MilitaryWeapDark/FX/P_Grenade_Explosion_01.P_Grenade_Explosion_01" _returnvalue)
      (`GameplayStatics.SpawnSoundAtLocation` "/Game/MilitaryWeapSilver/Sound/GrenadeLauncher/Cues/GrenadeLauncher_Explosion_Cue.GrenadeLauncher_Explosion_Cue" _returnvalue (struct) 1.0 1.0 0.0 null null)
      (`GameplayStatics.ApplyRadialDamage` :`BaseDamage` 30.0 :`Origin` (`self.K2_GetActorLocation`) :`DamageRadius` 250.0 :`DamageCauser` self :`InstigatedByController` null)
      (`self.K2_DestroyActor`))))

(fn `UserConstructionScript`)
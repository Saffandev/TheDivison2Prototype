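; BP_Bullet is a reusable projectile that waits hidden, motionless and non-colliding at the world origin until fired.
; FireBullet applies a velocity, enables cube collision and shows the actor, then StopBullet resets it after a short delay rather than destroying it.
; Overlapping a miss-detection sphere plays a whip-by sound and camera shake without stopping it.
; Any other overlap except another bullet resets it immediately.
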(event `self.ReceiveBeginPlay`
  (`self.StopBullet`))

(event `FireBullet`
  (params (Velocity :type "Vector Structure"))
  (set `MovementComponent.Velocity` Velocity (`self.ProjectileMovement`))
  (`PrimitiveComponent.SetCollisionEnabled` (`self.Cube`) "QueryAndPhysics")
  (`self.SetActorHiddenInGame` false)
  (`KismetSystemLibrary.Delay` 1.6)
  (`self.StopBullet`))

(event `StopBullet`
  (set `MovementComponent.Velocity` (0.0 0.0 0.0) (`self.ProjectileMovement`))
  (`PrimitiveComponent.SetCollisionEnabled` (`self.Cube`) "NoCollision")
  (`self.SetActorHiddenInGame` true)
  (`self.K2_SetActorLocation` (0.0 0.0 0.0)))

(event `self.Cube.OnComponentBeginOverlap`
  (params (OverlappedComponent :type "PrimitiveComponent Object Reference") (OtherActor :type "Actor Object Reference") (OtherComp :type "PrimitiveComponent Object Reference") (OtherBodyIndex :type Integer) (bFromSweep :type Boolean) (SweepResult :type "HitResult Structure (by ref)"))
  (bind _returnvalue (`GameplayStatics.GetObjectClass` OtherActor))
  (if (== _returnvalue "/Game/Blueprints/Bullets/BP_BulletMissDetectSpherer.BP_BulletMissDetectSpherer_C")
    (`GameplayStatics.SpawnSoundAtLocation` "/Game/MilitaryWeapSilver/Sound/Rifle/Cues/Rifle_Whip_Cue.Rifle_Whip_Cue" (`self.K2_GetActorLocation` OtherActor) (struct) 0.3 1.0 0.0 null null)
    (`PlayerCameraManager.StartCameraShake` :`self` (`PlayerController.PlayerCameraManager` (`GameplayStatics.GetPlayerController` 0)) :`ShakeClass` "/Game/Blueprints/Camera/CameraShake_BulletHit1.CameraShake_BulletHit1_C")
    (elif (not (== _returnvalue "BP_Bullet_C"))
      (`self.StopBullet`))))

(fn `UserConstructionScript`)
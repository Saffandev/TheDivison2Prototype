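; Bullet pool component that pre-spawns BP_Bullet actors and reuses them when shots are fired.
; BeginPlay fills the Bullets array with actors spawned at the owner's location.
; SpawnBullet moves the current bullet to the spawn point, fires it along Direction scaled by Speed, then advances a round-robin index that wraps at BulletCount.
; Bullet rotation derives from the SpawnPoint vector rather than Direction, and an invalid slot stalls the index.
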(event `self.ReceiveBeginPlay`
  (for _ (range (+ (`self.BulletCount`) 1))
    (bind _returnvalue (`|SpawnActorFromClass` "/Game/Blueprints/Bullets/BP_Bullet.BP_Bullet_C" (`KismetMathLibrary.MakeTransform` (`Actor.K2_GetActorLocation` (`self.GetOwner`))) "Undefined" "MultiplyWithRoot" null null))
    (`KismetArrayLibrary.Array_Add` (`self.Bullets`) _returnvalue)))

(event `SpawnBullet`
  (params (SpawnPoint :type "Vector Structure") (Direction :type "Vector Structure"))
  (bind _output (`|GetArrayItem` (`self.Bullets`) (`self.BulletIndex`)))
  (`/Engine/EditorBlueprintResources/StandardMacros.IsValid` _output
    (:`Is Valid`
      (`Actor.K2_SetActorLocationAndRotation` _output SpawnPoint (`KismetMathLibrary.Conv_VectorToRotator` SpawnPoint) false false)
      (`/Game/Blueprints/Bullets/BP_Bullet.FireBullet` _output (* Direction (`self.Speed`)))
      (bind _result (`/Engine/EditorBlueprintResources/StandardMacros.IncrementInt` (`self.BulletIndex`))
        (:`  `
          (if (>= _result (`self.BulletCount`))
            (set `self.BulletIndex` 0)))))))
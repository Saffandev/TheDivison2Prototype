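; BP_GunBasePlayer is the player's rifle, handling timer-driven firing, magazine ammo, reloading and hit markers.
; Each shot traces from camera, then from muzzle to the aimed point, so obstructions near the gun count.
; Fire also plays animations, spawns pooled bullets, trails, impacts and camera shake.
; Hits on damageable actors apply point damage, report AI damage events and flash the hit marker, while an empty magazine triggers a reload.
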(event Custom|Fire
  ;[0 0 0] Fire Logic
  (if (and (Variables|Default|GetbCanFire) (> (Variables|Default|GetCurrentMagCapacity) 0))
    (Variables|Default|SetAccuracyOverTime (Math|Float|Clamp(Float) (+ (Variables|Default|GetAccuracyOverTime) 0.04)))
    (if (< (stale _result) 5)
      (Utilities|FlowControl|Sequence
        (:then_0
          ;;[1 1 1] Trace
          (|Trace))
        (:then_1
          ;;[1 1 1] Animation
          (Components|Animation|PlayAnimation (Variables|Default|GetSkeletalMesh) "/Game/MilitaryWeapSilver/Weapons/Animations/Fire_Rifle_W.Fire_Rifle_W" false)
          (Animation|PlayAnimMontage (Variables|Default|GetGunOwner) (select (Variables|Default|GetADS) "/Game/AnimStarterPack/Montage/Fire_Rifle_Ironsights_Montage.Fire_Rifle_Ironsights_Montage" "/Game/AnimStarterPack/Montage/Fire_Rifle_Hip_Montage.Fire_Rifle_Hip_Montage") 1.0 "None"))
        (:then_2
          ;;[1 1 1] Spawning Bullets
          (Default|SpawnBullet (Variables|Default|GetUBulletPool) (Transformation|GetWorldLocation (Variables|Default|GetMuzzle)) (Math|Vector|Normalize (- (Variables|Default|GetTraceEndPoint) (Variables|Default|GetTraceStart\)))))
        (:then_3
          ;;[1 1 1] Visuals and sound
          (|Visuals))
        (:then_4
          ;;[1 1 1] Damage
          (|Damage))
        (:then_5
          (CameraShakes|StartCameraShake (Variables|/Script/Engine.PlayerController|GetPlayerCameraManager (Game|GetPlayerController 0)) "/Game/Blueprints/Camera/CameraShake_Fire.CameraShake_Fire_C" 1.0 "CameraLocal" "0, 0, 0"))
        (:then_6
          (Math|Integer|DecrementInt (Variables|Default|GetCurrentMagCapacity)
            (:%20%20
              (CallFunction|UpdateAmmoVisual)))))
      (else
        (Variables|Default|SetBrustCount 0)
        (Utilities|Time|ClearandInvalidateTimerbyHandle (Variables|Default|GetFireEvent))))
    (else
      (CallFunction|Reload))))

(event Custom|StopFire
  ;[1 1 1] Stop Firing
  (Utilities|Time|ClearandInvalidateTimerbyHandle (Variables|Default|GetInitFireEvent))
  (Utilities|Time|ClearandInvalidateTimerbyHandle (Variables|Default|GetFireEvent))
  (Variables|Default|SetBrustCount 0)
  (Variables|Default|SetAccuracyOverTime 0.0))

(event Custom|StartFire
  ;[1 1 1] Initiate Fire
  (bind _returnvalue (Utilities|Time|SetTimerbyFunctionName 0 "InitiateFire" 1.0 true))
  (Variables|Default|SetInitFireEvent _returnvalue))

(event Custom|InitiateFire
  (params (ADS :type Boolean))
  ;[1 1 1] Starting the weapon fire
  (CallFunction|Fire)
  (bind _returnvalue (Utilities|Time|SetTimerbyFunctionName 0 "Fire" 0.08 true))
  (Variables|Default|SetFireEvent _returnvalue))

(event Custom|Reload
  (if (< (Variables|Default|GetCurrentMagCapacity) (Variables|Default|GetMagSize))
    (Variables|Default|SetbCanFire false)
    (CallFunction|StopFire)
    (Components|Animation|PlayAnimation (Variables|Default|GetSkeletalMesh) "/Game/MilitaryWeapSilver/Weapons/Animations/Reload_Rifle_Ironsights_W.Reload_Rifle_Ironsights_W" false)
    (bind _returnvalue (Animation|PlayAnimMontage (Variables|Default|GetGunOwner) "/Game/AnimStarterPack/Montage/Reload_Rifle_Hip_Montage.Reload_Rifle_Hip_Montage" 1.0 "None"))
    (Utilities|FlowControl|Delay _returnvalue)
    (Variables|Default|SetCurrentMagCapacity (Variables|Default|GetMagSize))
    (CallFunction|UpdateAmmoVisual)
    (Variables|Default|SetbCanFire true)))

(event EventBeginPlay
  ;[1 1 1] begin play
  (Variables|Default|SetCurrentMagCapacity (Variables|Default|GetMagSize))
  (bind _returnvalue (UserInterface|CreateWidget "/Game/Widget/WBP_HitMarker.WBP_HitMarker_C"))
  (bind _output_get (Variables|Default|SetHitMarkerWidget _returnvalue))
  (UserInterface|Viewport|AddtoViewport _output_get 0)
  (bind _asbp_player (Utilities|Casting|CastToBP_Player (Components|GetOwner)))
  (Variables|Default|SetGunOwner _asbp_player)
  (CallFunction|UpdateAmmoVisual))

(fn ConstructionScript)

(fn DeathMarker
  (Default|DeathMarker (Variables|Default|GetHitMarkerWidget)))

(fn UpdateAmmoVisual
  (Default|UpdateAmmoinWidget (Variables|Default|GetGunOwner) (Variables|Default|GetCurrentMagCapacity)))
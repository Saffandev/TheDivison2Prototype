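; Base gun actor for AI characters, firing timed bursts at a rate and magazine size read from a weapon data asset.
; A looping timer drives Fire, which plays animations, then line-traces once, or repeatedly for shotguns.
; Traces not hitting the owner's class spawn pooled bullets, trail and impact effects, and point damage only the player.
; An empty magazine stops firing, sets the owner's combat state and refills after a montage.
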(event `self.ReceiveBeginPlay`
  ;[1 1 1] begin play
  (bind _asbp_ai (cast `/Game/AI/Blueprints/BP_AI` (`self.GetOwner`)))
  (bind _output_get (set `self.GunOwner` _asbp_ai))
  (set `self.AITraits` (`/Game/AI/Blueprints/BP_AI.AITraits` _output_get))
  (set `self.CurrentMagCount` (`/Game/AI/DataAssets/WeaponData/WeaponDataAssets.MagSize` (`self.WeaponDataAsset`)))
  (set `self.FireRateTimerValue` (/ 60.0 (`/Game/AI/DataAssets/WeaponData/WeaponDataAssets.FireRate` (`self.WeaponDataAsset`)))))

(event `StartFire`
  (params (FireDuration :type "Float (double-precision)"))
  (bind _returnvalue (/ (- FireDuration 1.0) (+ (/ (`KismetMathLibrary.RandomBool`) 2) 2.0)))
  ;[1 1 1] Initiate Fire
  (set `self.bIsFiring` true)
  (`KismetSystemLibrary.Delay` (/ (/ (`KismetMathLibrary.RandomBool`) 2) 5))
  (`self.InitiateFire`)
  (`KismetSystemLibrary.PrintString` (`KismetStringLibrary.Conv_DoubleToString` _returnvalue))
  (`KismetSystemLibrary.Delay` _returnvalue)
  (`KismetSystemLibrary.K2_ClearAndInvalidateTimerHandle` (`self.FireEvent`))
  (`KismetSystemLibrary.Delay` 1.8)
  (`self.InitiateFire`))

(event `StopFire`
  ;[1 1 1] Stop Firing
  (set `self.bIsFiring` false)
  (`KismetSystemLibrary.K2_ClearAndInvalidateTimerHandle` (`self.FireEvent`)))

(event `InitiateFire`
  ;[1 1 1] Starting the weapon fire
  (if (`self.bIsFiring`)
    (`self.Fire`)
    (bind _returnvalue (`KismetSystemLibrary.K2_SetTimerDelegate` (`|CreateDelegate` :!event `Fire`) (`self.FireRateTimerValue`) true))
    (set `self.FireEvent` _returnvalue)))

(event `Fire`
  (bind (_out_hit_bblockinghit _out_hit_binitialoverlap _out_hit_time _out_hit_distance _out_hit_location _out_hit_impactpoint _out_hit_normal _out_hit_impactnormal _out_hit_physmat _out_hit_hitactor) (`GameplayStatics.BreakHitResult` (`self.Out Hit`)))
  ;[0 0 0] Fire Logic
  (if (> (`self.CurrentMagCount`) 0)
    (bind _result (`/Engine/EditorBlueprintResources/StandardMacros.DecrementInt` (`self.CurrentMagCount`))
      (:`  `
        (`|ExecutionSequence`
          (:`then_0`
            ;;[1 1 1] Animation
            (`self.Animation`))
          (:`then_1`
            (if (`|EnumEquality` (`/Game/AI/DataAssets/WeaponData/WeaponDataAssets.WeaponType` (`self.WeaponDataAsset`)) "Shotgun")
              (for _ (range 16)
                (`|ExecutionSequence` :!label _label
                  (:`then_0`
                    ;;[1 1 1] Trace
                    (`self.GunTrace`))
                  (:`then_1`
                    (if (!= (`GameplayStatics.GetObjectClass` _out_hit_hitactor) (`GameplayStatics.GetObjectClass` (`self.GunOwner`)))
                      (`|ExecutionSequence`
                        (:`then_0`
                          ;;[1 1 1] Spawning Bullets
                          (`self.SpawnBullet`))
                        (:`then_1`
                          ;;[1 1 1] Visuals and sound
                          (`self.VisualsAndSound`))
                        (:`then_2`
                          ;;[1 1 1] Damage
                          (`self.Damage`)))))))
              (else
                (goto _label)))))))
    (else
      (`self.Reload`))))

(event `Reload`
  (bind _aifireanim (`/Game/AI/DataAssets/WeaponData/WeaponDataAssets.AIFireAnim` (`self.WeaponDataAsset`)))
  (`/Game/AI/Blueprints/BP_AI.SetCombatState` (`self.GunOwner`) "NewEnumerator4")
  (`self.StopFire`)
  (`KismetSystemLibrary.Delay` 0.3)
  (`/Engine/EditorBlueprintResources/StandardMacros.IsValid` _aifireanim
    (:`Is Valid`
      (`|PlayMontage` (`Character.Mesh` (`self.GunOwner`)) _aifireanim
        (:`OnCompleted`
          (`KismetSystemLibrary.Delay` 0.2)
          (set `self.CurrentMagCount` (`/Game/AI/DataAssets/WeaponData/WeaponDataAssets.MagSize` (`self.WeaponDataAsset`)))
          (`/Game/AI/Blueprints/BP_AI.SetCombatState` (`self.GunOwner`) "NewEnumerator3"))))))

(fn `Animation`
  (bind (_aitraits_aitype _aitraits_bcantakecover _aitraits_bcanthrowgrenade _aitraits_walkingspeed _aitraits_sprintspeed _aitraits_adsspeed _aitraits_health _aitraits_advancingtime _aitraits_stunthreshold _aitraits_stunduration _aitraits_fireduration _aitraits_firegap _aitraits_maxcombatrange _aitraits_mincombatrange _aitraits_gunclass _aitraits_behaviortree _aitraits_firemontage) (break `AITraits` (`self.AITraits`)))
  (bind _fireanim (`/Game/AI/DataAssets/WeaponData/WeaponDataAssets.FireAnim` (`self.WeaponDataAsset`)))
  (`/Engine/EditorBlueprintResources/StandardMacros.IsValid` _fireanim
    (:`Is Valid`
      (`SkeletalMeshComponent.PlayAnimation` (`self.SkeletalMesh`) _fireanim false)
      (`/Engine/EditorBlueprintResources/StandardMacros.IsValid` _aitraits_firemontage
        (:`Is Valid`
          (`Character.PlayAnimMontage` (`self.GunOwner`) _aitraits_firemontage 1.0 "None"))))))

(fn `Damage`
  (locals (DamagedActor :type "Actor Object Reference"))
  (bind (_out_hit_bblockinghit _out_hit_binitialoverlap _out_hit_time _out_hit_distance _out_hit_location _out_hit_impactpoint _out_hit_normal _out_hit_impactnormal _out_hit_physmat _out_hit_hitactor) (`GameplayStatics.BreakHitResult` (`self.Out Hit`)))
  (bind (_bblockinghit _binitialoverlap _time _distance _location _impactpoint _normal _impactnormal _physmat _hitactor _hitcomponent _hitbonename _bonename _hititem _elementindex _faceindex _tracestart) (`GameplayStatics.BreakHitResult` (`self.Out Hit`)))
  (set `local.DamagedActor` _out_hit_hitactor)
  (if (`self.bTraceHit`)
    (`/Engine/EditorBlueprintResources/StandardMacros.IsValid` (`local.DamagedActor`)
      (:`Is Valid`
        (if (and (== (`local.DamagedActor`) (`GameplayStatics.GetPlayerPawn` 0)) (`Actor.bCanBeDamaged` (`local.DamagedActor`)))
          (`GameplayStatics.ApplyPointDamage` (`local.DamagedActor`) 1.0 (`KismetMathLibrary.Normal` (- _impactpoint _tracestart)) (`self.Out Hit`) null self))))))

(fn `GunTrace`
  (bind _returnvalue (- 1.0 (`/Game/AI/DataAssets/WeaponData/WeaponDataAssets.Accuracy` (`self.WeaponDataAsset`))))
  (set `self.TraceEndPoint` (+ (`self.K2_GetActorLocation` (`self.GetOwner`)) (* (`KismetMathLibrary.Normal` (- (`AIController.GetFocalPoint` (`AIBlueprintHelperLibrary.GetAIController` (`self.GetOwner`))) (`SceneComponent.K2_GetComponentLocation` (`self.Arrow`)))) 10000) (`KismetMathLibrary.MakeVector` 0.0 (* (`KismetMathLibrary.RandomFloatInRange` -1.0 1.0) 350.0 _returnvalue) (* (`KismetMathLibrary.RandomFloatInRange` -1.0 1.0) 350.0 _returnvalue))))
  (bind (_outhit _returnvalue_2) (`KismetSystemLibrary.LineTraceSingle` (`SceneComponent.K2_GetComponentLocation` (`self.Arrow`)) (`self.TraceEndPoint`) "TraceTypeQuery1" false (`|MakeArray` self (`self.GunOwner`) :!type "Actor Object Reference") "None" true (struct :`R` 1.0 :`A` 1.0) (struct :`G` 1.0 :`A` 1.0) 1.0))
  (set `self.Out Hit` _outhit)
  (set `self.bTraceHit` _returnvalue_2))

(fn `SpawnBullet`
  (`/Game/Blueprints/Bullets/UBulletPool.SpawnBullet` (`self.UBulletPool`) (`SceneComponent.K2_GetComponentLocation` (`self.Arrow`)) (`KismetMathLibrary.Normal` (- (`self.TraceEndPoint`) (`SceneComponent.K2_GetComponentLocation` (`self.Arrow`))))))

(fn `UserConstructionScript`)

(fn `VisualsAndSound`
  (locals (WeaponTrailEndPoint :type "Vector Structure"))
  (bind (_bblockinghit _binitialoverlap _time _distance _location _impactpoint _normal _impactnormal) (`GameplayStatics.BreakHitResult` (`self.Out Hit`)))
  (bind (_bblockinghit_2 _binitialoverlap_2 _time_2 _distance_2 _location_2 _impactpoint_2 _normal_2 _impactnormal_2 _physmat _hitactor) (`GameplayStatics.BreakHitResult` (`self.Out Hit`)))
  (set `local.WeaponTrailEndPoint` (select `bool` (`self.bTraceHit`) :`false` (`self.TraceEndPoint`) :`true` (`.ImpactPoint` (`GameplayStatics.BreakHitResult` (`self.Out Hit`)))))
  (bind _returnvalue (`GameplayStatics.SpawnEmitterAtLocation` "/Game/Particles/P_AssaultRifle_Trail.P_AssaultRifle_Trail" (`SceneComponent.K2_GetComponentLocation` (`self.Arrow`))))
  (`FXSystemComponent.SetVectorParameter` _returnvalue "ShockBeamEnd" (`local.WeaponTrailEndPoint`))
  (if _bblockinghit_2
    (`/Engine/EditorBlueprintResources/StandardMacros.IsValid` _hitactor
      (:`Is Valid`
        (if (not (`Actor.bCanBeDamaged` _hitactor))
          (`GameplayStatics.SpawnEmitterAtLocation` "/Game/MilitaryWeapSilver/FX/P_Impact_Stone_Large_01.P_Impact_Stone_Large_01" _impactpoint (`KismetMathLibrary.Conv_VectorToRotator` _impactnormal) (0.4 0.4 0.4))
          (`GameplayStatics.PlaySoundAtLocation` "/Game/MilitaryWeapSilver/Sound/Rifle/Cues/Rifle_ImpactSurface_Cue.Rifle_ImpactSurface_Cue" _impactpoint (struct) 0.5 1.0 0.0 null null null null))))))
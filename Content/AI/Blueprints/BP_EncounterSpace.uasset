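; Encounter volume that coordinates the AI inside its box for group combat and grenade throws.
; Shortly after BeginPlay it caches overlapping AI and covers and registers itself with each AI controller.
; CombatStarted sets their combat state and starts a looping grenade timer, gated by a condition whose distance check is unwired.
; The throw goes to the first eligible in-cover AI with a clear trace from the player's last known location.
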(event `self.ReceiveBeginPlay`
  ;[1 1 1] Begin Play
  (`KismetSystemLibrary.Delay` 0.5)
  (`self.SaveAI`)
  (set `self.OverlappingCovers` (`PrimitiveComponent.GetOverlappingActors` (`self.Box`) "/Game/AI/Blueprints/BP_Cover.BP_Cover_C")))

(event `InitiateGrenading`
  ;[1 1 1] Grende
  (bind _returnvalue (`KismetSystemLibrary.K2_SetTimerDelegate` (delegate `CheckForGrenadeThrow`) (`KismetMathLibrary.Conv_IntToDouble` (`KismetMathLibrary.RandomIntegerInRange` 15 20)) true))
  (set `self.GrenadeInitTimer` _returnvalue))

(event `CheckForGrenadeThrow`
  ;[1 1 1] Grende
  (if (< (`KismetMathLibrary.Vector_DistanceSquared` (`BlackboardComponent.GetValueAsVector` (`AIBlueprintHelperLibrary.GetBlackboard` (`AIBlueprintHelperLibrary.GetAIController` (`|GetArrayItem` (`self.OverlappingAIs`)))) "PlayerLastKnownLocation") (`self.K2_GetActorLocation` (`GameplayStatics.GetPlayerPawn` 0))) 90000.0)
    (`self.SelectAIForGrenadeToss`)))

(event `CombatEnded`
  ;[1 1 1] Combad Ended
  (`KismetSystemLibrary.K2_ClearAndInvalidateTimerHandle` (`self.GrenadeInitTimer`)))

(event `SelectForInvestigation`
  ;[1 1 1] Investigation(Not doing it right now)
  (bind _returnvalue (`EnvQueryManager.RunEQSQuery` "/Game/AI/BT/EQS_ClosestAI.EQS_ClosestAI" (`GameplayStatics.GetPlayerPawn` 0) "RandomBest5Pct"))
  (add `EnvQueryInstanceBlueprintWrapper.OnQueryFinishedEvent` _returnvalue (delegate `OnQueryFinished_SelectAIForInvestigation`)))

(event `OnQueryFinished_SelectAIForInvestigation`
  (params (QueryInstance :type "EnvQueryInstanceBlueprintWrapper Object Reference") (QueryStatus :type "EEnvQueryStatus Enum" :default "Processing"))
  ;[1 1 1] Investigation(Not doing it right now)
  (bind _resultactors (`EnvQueryInstanceBlueprintWrapper.GetQueryResultsAsActors` QueryInstance))
  (bind _asbp_aicontroller (cast `/Game/AI/Blueprints/BP_AIController` (`AIBlueprintHelperLibrary.GetAIController` (`|GetArrayItem` _resultactors))))
  (`/Game/AI/Blueprints/BP_AIController.SetCombatState` _asbp_aicontroller "NewEnumerator5"))

(fn `AIDead`
  (params (Item :type "Actor Object Reference (by ref)"))
  (`KismetArrayLibrary.Array_RemoveItem` (`self.OverlappingAIs`) Item))

(fn `CombatStarted`
  (`|ExecutionSequence`
    (:`then_0`
      (for _array_element (`self.OverlappingAIs`)
        (bind _asbp_aicontroller (cast `/Game/AI/Blueprints/BP_AIController` (`AIBlueprintHelperLibrary.GetAIController` _array_element)))
        (`/Game/AI/Blueprints/BP_AIController.SetCombatState` _asbp_aicontroller "NewEnumerator3")))
    (:`then_1`
      (`self.InitiateGrenading`))))

(fn `NewFunction`
  (returns (reservedLocations :type "Array of Vector Structure"))
  (for _array_element (`self.SavedAIController`)
    (`KismetArrayLibrary.Array_Add` (`self.reservedLocations`) (`BlackboardComponent.GetValueAsVector` (`AIBlueprintHelperLibrary.GetBlackboard` _array_element) "ReservedLocation")))
  (return (`self.reservedLocations`)))

(fn `SaveAI`
  (bind _output_get (set `self.OverlappingAIs` (`PrimitiveComponent.GetOverlappingActors` (`self.Box`) "/Game/AI/Blueprints/BP_AI.BP_AI_C")))
  (for _array_element _output_get
    (bind _asbp_aicontroller (cast `/Game/AI/Blueprints/BP_AIController` (`AIBlueprintHelperLibrary.GetAIController` _array_element)))
    (`/Game/AI/Blueprints/BP_AIController.SaveEncounterS[ace` _asbp_aicontroller self)
    (`KismetArrayLibrary.Array_Add` (`self.SavedAIController`) _asbp_aicontroller)))

(fn `SelectAIForGrenadeToss`
  (locals (LastKnownLoc :type "Vector Structure") (AILoc :type "Vector Structure") (ActorAI :type "Actor Object Reference") (Blackboard :type "BlackboardComponent Object Reference"))
  (for _array_element (`self.OverlappingAIs`)
    (set `local.ActorAI` _array_element)
    (set `local.AILoc` (+ (`SceneComponent.K2_GetComponentLocation` (`self.GetComponentByClass` (`local.ActorAI`) "/Script/Engine.SkeletalMeshComponent")) (0.0 0.0 155.0)))
    (set `local.Blackboard` (`AIBlueprintHelperLibrary.GetBlackboard` (`AIBlueprintHelperLibrary.GetAIController` (`local.ActorAI`))))
    (`local.Blackboard`
      (:`then`
        (if (`BlackboardComponent.GetValueAsBool` (`local.Blackboard`) "bCanThrowGrenade")
          (if (`BlackboardComponent.GetValueAsBool` (`local.Blackboard`) "bInCover")
            (set `local.LastKnownLoc` (`BlackboardComponent.GetValueAsVector` (`local.Blackboard`) "PlayerLastKnownLocation"))
            (if (< (`KismetMathLibrary.Vector_Distance` (`local.LastKnownLoc`) (`local.AILoc`)) 4500.0)
              (bind (_outhit _returnvalue) (`KismetSystemLibrary.LineTraceSingle` (`local.LastKnownLoc`) (`local.AILoc`) "TraceTypeQuery1" false (`|MakeArray` (`GameplayStatics.GetPlayerPawn` 0) (`local.ActorAI`) :!type "Actor Object Reference") "ForDuration" true (struct :`R` 1.0 :`A` 1.0) (struct :`G` 1.0 :`A` 1.0) 10.0))
              (if (not _returnvalue)
                (bind _asbp_ai (cast `/Game/AI/Blueprints/BP_AI` (`local.ActorAI`)))
                (`/Game/AI/Blueprints/BP_AI.initGrenadeThrow` _asbp_ai (`local.LastKnownLoc`))
                (return))))))
      (:`else`))))

(fn `UserConstructionScript`)
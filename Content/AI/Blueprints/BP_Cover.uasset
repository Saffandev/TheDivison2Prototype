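; AI cover actor that picks a cover point and peek point against the player's last known location from the blackboard.
; Candidates must lie behind the cover relative to the player, by distance and angle.
; Crouch cover takes the two farthest, prefers more clear line traces to the player, then adds the nearest peek point.
; Standing cover picks the peek point first but always reports invalid; Blueprint point generation is disconnected.
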(event `self.Generate`
  ;[1 1 1] generating Cover points
)

(event `self.SetCoverVisMaterial`
  (`PrimitiveComponent.SetMaterial` (`self.CoverVisualBox`) 0 (select `bool` (`self.bIsStandingCover`) :`false` "/Game/Materials/MI_color2.MI_color2" :`true` "/Game/Materials/MI_color1.MI_color1" :!type "MaterialInterface Object Reference")))

(fn `BestCover`
  (params (PlayerLastKnownLocation :type "Vector Structure"))
  (returns (CoverPoint :type "Vector Structure") (PeakPoint :type "Vector Structure") (bHasValidPoint :type Boolean))
  (locals (Peak :type "Array of Vector Structure") (Cover :type "Array of Vector Structure") (TempCover :type "Vector Structure" :default (0.0 0.0 0.0)) (TempPeak :type "Vector Structure" :default (0.0 0.0 0.0)))
  (set `self.Player Last Known Location` PlayerLastKnownLocation)
  (if (`self.bIsStandingCover`)
    (bind (_peak_point _coverpoint) (`self.PeakCoverTesting`))
    (return _coverpoint _peak_point false)
    (else
      (set `local.Peak` (`self.GetPeakPoitns`))
      (set `local.Cover` (`self.GetCrouchPoints`))
      (bind _coverlocation (`self.GiveCoverPoint` (`local.Cover`)))
      (bind _output_get (set `local.TempCover` _coverlocation))
      (if (!= _output_get (0.0 0.0 0.0))
        (bind _peakpoint (`self.Give Peak Points` (`local.TempCover`) (`local.Peak`)))
        (set `local.TempPeak` _peakpoint)
        (return (`local.TempCover`) (`local.TempPeak`) true)
        (else
          (return (0.0 0.0 0.0) (0.0 0.0 0.0) false))))))

(fn `bHasValidCoverPoints`
  (params (CoverRequester :type "Actor Object Reference"))
  (returns (ReturnValue :type Boolean))
  (bind (_coverpoint _peakpoint _bhasvalidpoint) (`self.BestCover` (`BlackboardComponent.GetValueAsVector` (`AIBlueprintHelperLibrary.GetBlackboard` (`AIBlueprintHelperLibrary.GetAIController` CoverRequester)) "PlayerLastKnownLocation")))
  (if _bhasvalidpoint
    (set `self.SavedCoverPoint` _coverpoint)
    (set `self.SavedPeakPoint` _peakpoint))
  (return _bhasvalidpoint))

(fn `CalculateLoopIncrement`
  (params (A :type "Float (double-precision)"))
  (returns (ReturnValue :type "Float (double-precision)"))
  (return (`KismetMathLibrary.FMax` (/ 1.0 (`KismetMathLibrary.Conv_IntToDouble` (`KismetMathLibrary.FFloor` (/ A 100.0)))) 0.5)))

(fn `CheckForPointValidity`
  (params (Point1 :type "Vector Structure"))
  (returns (bValidPoint :type Boolean) (ReturnValue :type "Vector Structure"))
  (locals (Point :type "Vector Structure") (PointInWorldSpace :type "Vector Structure" :default (0.0 0.0 0.0)))
  (bind _pointinworldspace (`local.PointInWorldSpace`))
  (bind (_projectedlocation _returnvalue) (`NavigationSystemV1.K2_ProjectPointToNavigation` (`local.PointInWorldSpace`) null "/Game/AI/Navigation/CoverNavFilter.CoverNavFilter_C" (50.0 50.0 200.0)))
  (set `local.Point` Point1)
  (set `local.PointInWorldSpace` (`KismetMathLibrary.TransformLocation` (`self.GetTransform`) (`local.Point`)))
  (bind (_outhit _returnvalue_2) (`KismetSystemLibrary.SphereTraceSingle` _pointinworldspace _pointinworldspace 10.0 "TraceTypeQuery1" false (`|MakeArray` self :!type "Actor Object Reference")))
  (if _returnvalue_2
    (return false (0.0 0.0 0.0))
    (elif _returnvalue
      (bind _output_get (set `local.Point` _projectedlocation))
      (return true (`KismetMathLibrary.InverseTransformLocation` (`self.GetTransform`) _output_get))
      (else
        (return false (0.0 0.0 0.0))))))

(fn `CloserToPlayer b/w2`
  (params (Point1 :type "Vector Structure") (Point2 :type "Vector Structure"))
  (returns (ReturnValue :type Boolean))
  (bind _player_last_known_location (`self.Player Last Known Location`))
  (return (< (`KismetMathLibrary.Vector_DistanceSquared` (`local.Point1`) _player_last_known_location) (`KismetMathLibrary.Vector_DistanceSquared` _player_last_known_location (`local.Point2`)))))

(fn `CoverValidity`
  (params (CoverPoint :type "Vector Structure"))
  (returns (ReturnValue :type Boolean))
  (bind (_x _y) (`KismetMathLibrary.BreakVector3f` (`local.CoverPoint`)))
  (bind (_x_2 _y_2) (`KismetMathLibrary.BreakVector3f` (`self.Player Last Known Location`)))
  (if (> (`KismetMathLibrary.Vector_DistanceSquared` (`local.CoverPoint`) (`self.Player Last Known Location`)) (`KismetMathLibrary.Vector_DistanceSquared` (`self.K2_GetActorLocation`) (`self.Player Last Known Location`)))
    (return (> (`KismetMathLibrary.DegAcos` (`KismetMathLibrary.Dot_VectorVector` (`KismetMathLibrary.Normal` (- (`KismetMathLibrary.MakeVector` _x _y (`.Z` (`KismetMathLibrary.BreakVector3f` (`self.K2_GetActorLocation`)))) (`self.K2_GetActorLocation`))) (`KismetMathLibrary.Normal` (- (`KismetMathLibrary.MakeVector` _x_2 _y_2 (`.Z` (`KismetMathLibrary.BreakVector3f` (`self.K2_GetActorLocation`)))) (`self.K2_GetActorLocation`))))) 120.0))
    (else
      (return false))))

(fn `CreateCoverPoints`
  (params (PeakPoint :type "Vector3f Structure"))
  (bind (_x _y _z) (`KismetMathLibrary.BreakVector3f` (`local.PeakPoint`)))
  (bind (_x_2 _y_2 _z_2) (`KismetMathLibrary.BreakVector3f` (`local.PeakPoint`)))
  (bind (_returnvalue_x _returnvalue_y) (`KismetMathLibrary.BreakVector` (`BoxComponent.GetUnscaledBoxExtent` (`self.CoverBox`))))
  (bind _returnvalue_x_2 (`KismetMathLibrary.BreakVector` (`BoxComponent.GetUnscaledBoxExtent` (`self.CoverBox`))))
  (if (>= (- _returnvalue_x_2 70.0) 100.0)
    (bind (_bvalidpoint _returnvalue) (`self.CheckForPointValidity` (`KismetMathLibrary.MakeVector` (+ (* (`self.temp`) (`KismetMathLibrary.SelectFloat` 1.0 -1.0 (> _x_2 0.0))) _x_2) _y_2 (+ _z_2 30.0))))
    (if _bvalidpoint
      (`KismetArrayLibrary.Array_Add` (`self.CoverPointsBP`) _returnvalue)))
  (if (>= (- _returnvalue_y 70.0) 100.0)
    (bind (_bvalidpoint_2 _returnvalue_2) (`self.CheckForPointValidity` (`KismetMathLibrary.MakeVector` _x (+ _y (* (`KismetMathLibrary.SelectFloat` 1.0 -1.0 (> _y 0.0)) (`self.temp`))) (+ _z 30.0))))
    (if _bvalidpoint_2
      (`KismetArrayLibrary.Array_Add` (`self.CoverPointsBP`) _returnvalue_2))))

(fn `CreatePoint`
  (returns (ReturnValue :type "Vector Structure"))
  (bind _coverpointscale (`self.CoverPointScale`))
  (bind (_x _y) (`KismetMathLibrary.BreakVector3f` (`BoxComponent.BoxExtent` (`self.CoverBox`))))
  (return (+ (`KismetMathLibrary.MakeVector` (* _x (`self.X`) 1.0 _coverpointscale) (* _y (`self.Y`) 1.0 _coverpointscale)) (0.0 0.0 0.0))))

(fn `Farthese2Points`
  (params (Array :type "Array of Vector Structure") (DistanceFrom :type "Vector Structure") (`bFarthest?` :type Boolean))
  (returns (CoverPoint1 :type "Vector Structure") (CoverPoint2 :type "Vector Structure"))
  (locals (ArrayElem :type "Vector Structure") (Distance :type "Float (double-precision)") (CoverDistance2 :type "Float (double-precision)") (CoverDistance :type "Float (double-precision)") (LCoverLocation2 :type "Vector Structure") (LCoverLocation :type "Vector Structure"))
  (bind _coverdistance (`local.CoverDistance`))
  (bind _distance (`local.Distance`))
  (bind _coverdistance2 (`local.CoverDistance2`))
  (bind _coverdistance_2 (`local.CoverDistance`))
  (bind _distance_2 (`local.Distance`))
  (set `local.CoverDistance` (select `bool` `bFarthest?` :`false` 100000000.0))
  (for _array_element Array
    (bind _output_get (set `local.ArrayElem` _array_element))
    (if (`self.CoverValidity` _output_get)
      (set `local.Distance` (`KismetMathLibrary.Vector_DistanceSquared` (`local.ArrayElem`) (`local.DistanceFrom`)))
      (if (select `bool` (`local.bFarthest?`) :`false` (< _distance_2 _coverdistance) :`true` (> _distance_2 _coverdistance))
        (set `local.CoverDistance2` (`local.CoverDistance`))
        (set `local.LCoverLocation2` (`local.LCoverLocation`))
        (set `local.CoverDistance` (`local.Distance`))
        (set `local.LCoverLocation` (`local.ArrayElem`))
        (elif (select `bool` (`local.bFarthest?`) :`false` (and (< _distance _coverdistance2) (> _coverdistance2 _coverdistance_2)) :`true` (and (> _distance _coverdistance2) (< _coverdistance2 _coverdistance_2)))
          (set `local.CoverDistance2` (`local.Distance`))
          (set `local.LCoverLocation2` (`local.ArrayElem`))))))
  (return (`local.LCoverLocation`) (`local.LCoverLocation2`)))

(fn `FloorVector`
  (params (InVector :type "Vector Structure"))
  (returns (OutVector :type "Vector Structure"))
  (bind (_x _y _z) (`KismetMathLibrary.BreakVector3f` InVector))
  (return (`KismetMathLibrary.MakeVector` (`KismetMathLibrary.Conv_IntToDouble` (`KismetMathLibrary.FFloor` _x)) (`KismetMathLibrary.Conv_IntToDouble` (`KismetMathLibrary.FFloor` _y)) (`KismetMathLibrary.Conv_IntToDouble` (`KismetMathLibrary.FFloor` _z)))))

(fn `Give Peak Points`
  (params (CoverPointLocation :type "Vector Structure") (Array :type "Array of Vector Structure"))
  (returns (PeakPoint :type "Vector Structure"))
  (locals (PeakDistance1 :type "Float (double-precision)" :default 1000000.0) (PeakPoint1 :type "Vector Structure") (`PeakDistance 2` :type "Float (double-precision)" :default 1000000.0) (PeakPoint2 :type "Vector Structure") (ArrayElem :type "Vector Structure") (Distance :type "Float (double-precision)" :default 0.0))
  (bind _returnvalue (`KismetMathLibrary.Vector_Distance` (`local.ArrayElem`) (`local.CoverPointLocation`)))
  (for _array_element Array
    (set `local.ArrayElem` _array_element)
    (if (< _returnvalue (`local.PeakDistance1`))
      (set `local.PeakDistance1` _returnvalue)
      (set `local.PeakPoint1` (`local.ArrayElem`))))
  (return (`local.PeakPoint1`)))

(fn `GiveCoverPoint`
  (params (Array :type "Array of Vector Structure"))
  (returns (CoverLocation :type "Vector Structure"))
  (locals (Cover1 :type "Vector Structure") (Cover2 :type "Vector Structure"))
  (bind _returnvalue (!= (`local.Cover1`) (0.0 0.0 0.0)))
  (if (> (`KismetArrayLibrary.Array_Length` Array) 1)
    (bind (_coverpoint1 _coverpoint2) (`self.Farthese2Points` (`local.Array`) (`self.Player Last Known Location`) true))
    (set `local.Cover1` _coverpoint1)
    (set `local.Cover2` _coverpoint2)
    (if (and _returnvalue (!= (`local.Cover2`) (0.0 0.0 0.0)))
      (bind _finalcoverpoint (`self.SelectBestCrouchCoverPoint` (`local.Cover1`) (`local.Cover2`)))
      (return _finalcoverpoint)
      (elif _returnvalue
        (return (`local.Cover1`))
        (else
          (return (`local.Cover1`)))))
    (else
      (return (`|GetArrayItem` Array)))))

(fn `HitCountForCrouchCover`
  (params (CoverPoint :type "Vector Structure"))
  (returns (HitCount1 :type Integer))
  (locals (HitCount :type Integer))
  (if (`self.CoverValidity` CoverPoint)
    (for _array_element (`self.TestingArray`)
      (bind (_outhit _returnvalue) (`KismetSystemLibrary.LineTraceSingle` (+ (`local.CoverPoint`) _array_element) (+ (`self.Player Last Known Location`) (0.0 0.0 50.0)) "TraceTypeQuery1" false (`|MakeArray` (`GameplayStatics.GetPlayerPawn` 0) self (`self.GetOwner`) :!type "Actor Object Reference")))
      (if (not _returnvalue)
        (`/Engine/EditorBlueprintResources/StandardMacros.IncrementInt` (`local.HitCount`)))))
  (return (`local.HitCount`)))

(fn `PeakCoverTesting`
  (returns (`Peak Point` :type "Vector Structure") (CoverPoint :type "Vector Structure"))
  (locals (LocalPeakPoints :type "Array of Vector Structure") (FarthestPeakPoint :type "Vector Structure") (Distance :type "Float (double-precision)" :default 0.0) (FinalPeakPoint :type "Vector Structure") (ClosestPeakPoint :type "Vector Structure"))
  (set `local.LocalPeakPoints` (`self.GetPeakPoitns`))
  (if (> (`KismetArrayLibrary.Array_Length` (`self.GetPeakPoitns`)) 2)
    (bind _peakpoint (`self.Give Peak Points` (`self.Player Last Known Location`) (`self.GetPeakPoitns`)))
    (set `local.ClosestPeakPoint` _peakpoint)
    (`KismetArrayLibrary.Array_RemoveItem` (`local.LocalPeakPoints`) (`local.ClosestPeakPoint`))
    (bind _coverpoint1 (`self.Farthese2Points` (`local.LocalPeakPoints`) (`self.Player Last Known Location`) true))
    (`KismetArrayLibrary.Array_RemoveItem` (`local.LocalPeakPoints`) _coverpoint1))
  (if (> (`KismetArrayLibrary.Array_Length` (`local.LocalPeakPoints`)) 1)
    (bind _coverpoint1_2 (`self.Farthese2Points` (`local.LocalPeakPoints`) (`self.Player Last Known Location`) true))
    (set `local.FinalPeakPoint` _coverpoint1_2)
    (else
      (set `local.FinalPeakPoint` (`|GetArrayItem` (`local.LocalPeakPoints`)))))
  (bind (_coverpoint1_3 _coverpoint2) (`self.Farthese2Points` (`self.GetCrouchPoints`) (`local.FinalPeakPoint`)))
  (return (`local.FinalPeakPoint`) (select `bool` (`self.CloserToPlayer b/w2` _coverpoint1_3 _coverpoint2) :`false` _coverpoint1_3 :`true` _coverpoint2)))

(fn `SelectBestCrouchCoverPoint`
  (params (CoverPoint1 :type "Vector Structure") (CoverPoint2 :type "Vector Structure"))
  (returns (FinalCoverPoint :type "Vector Structure"))
  (locals (HitCount1 :type Integer :default 0) (HitCount2 :type Integer :default 0) (FinalCover :type "Vector Structure"))
  (bind _hitcount1 (`self.HitCountForCrouchCover` CoverPoint1))
  (set `local.HitCount1` _hitcount1)
  (bind _hitcount1_2 (`self.HitCountForCrouchCover` CoverPoint2))
  (set `local.HitCount2` _hitcount1_2)
  (if (== (+ (`local.HitCount1`) (`local.HitCount2`)) 0)
    (return (0.0 0.0 0.0))
    (else
      (`/Engine/EditorBlueprintResources/StandardMacros.CompareInt` (`local.HitCount1`) (`local.HitCount2`)
        (:`>`
          (set `local.FinalCover` (`local.CoverPoint1`) :!label _label))
        (:`==`
          (goto _label))
        (:`<`
          (set `local.FinalCover` (`local.CoverPoint2`))))
      (return (`local.FinalCover`)))))

(fn `UserConstructionScript`
  (`self.GenerateCoverShape`))
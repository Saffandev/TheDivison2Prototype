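; AI cover-box actor meant to supply cover and peek points against the player's last known location, with standing or crouch variants shown by material.
; Generate sizes two nav modifiers from CoverBox, rebuilds navigation and scales the cube.
; Helpers validate points by sphere trace and navmesh projection, and rank them by distance and line traces.
; Point generation and selection are largely disconnected: BestCover's standing branch calls an empty PeakCoverTesting.
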(event `self.ReceiveBeginPlay`
  ;[1 1 1] Converting Point to world space
)

(event `self.Generate`
  (bind _boxextent (`BoxComponent.BoxExtent` (`self.CoverBox`)))
  (bind (_returnvalue_x _returnvalue_y) (`KismetMathLibrary.BreakVector` (/ _boxextent 3.5)))
  ;[1 1 1] generating Cover points
  (`self.SetNavModifierExtent` (`self.CoverNavModifier`) (+ (/ (`BoxComponent.BoxExtent` (`self.CoverBox`)) 2.0) 60))
  (`self.SetNavModifierExtent` (`self.NullNavModifier`) (`KismetMathLibrary.MakeVector` _returnvalue_x _returnvalue_y (`.Z` (`KismetMathLibrary.BreakVector3f` _boxextent))))
  (`KismetSystemLibrary.ExecuteConsoleCommand` "RebuildNavigation" null)
  (`|ExecutionSequence`
    (:`then_0`
      (set `self.InitActorRotaion` (`self.K2_GetActorRotation`)))
    (:`then_1`
      (`SceneComponent.SetWorldScale3D` (`self.Cube`) (/ (`BoxComponent.BoxExtent` (`self.CoverBox`)) 100.0)))))

(event `CoverPointTesting`)

(fn `BestCover`
  (params (PlayerLastKnownLocation :type "Vector Structure"))
  (returns (CoverPoint :type "Vector Structure") (PeakPoint :type "Vector Structure"))
  (locals (Peak :type "Array of Vector Structure") (Cover :type "Array of Vector Structure") (TempCover :type "Vector Structure" :default (0.0 0.0 0.0)) (TempPeak :type "Vector Structure" :default (0.0 0.0 0.0)))
  (set `self.Player Last Known Location` PlayerLastKnownLocation)
  (if (`self.bIsStandingCover`)
    (bind (_peak_point _coverpoint) (`self.PeakCoverTesting`))
    (return _coverpoint _peak_point)))

(fn `CalculateLoopIncrement`
  (params (A :type "Float (double-precision)"))
  (returns (ReturnValue :type "Float (double-precision)"))
  (return (`KismetMathLibrary.FMax` (/ 1.0 (`KismetMathLibrary.Conv_IntToDouble` (`KismetMathLibrary.FFloor` (/ A 100.0)))) 0.5)))

(fn `CheckForPointValidity`
  (params (Point1 :type "Vector Structure"))
  (returns (bValidPoint :type Boolean) (ReturnValue :type "Vector Structure"))
  (locals (Point :type "Vector Structure") (PointInWorldSpace :type "Vector Structure" :default (0.0 0.0 0.0)))
  (bind _pointinworldspace (`local.PointInWorldSpace`))
  (bind (_projectedlocation _returnvalue) (`NavigationSystemV1.K2_ProjectPointToNavigation` (`local.PointInWorldSpace`) null "/Game/AI/Navigation/CoverNavFilter.CoverNavFilter_C" (50.0 50.0 200.0)))
  (set `local.Point` Point1)
  (set `local.PointInWorldSpace` (`KismetMathLibrary.TransformLocation` (`self.GetTransform`) (`local.Point`)))
  (bind (_outhit _returnvalue_2) (`KismetSystemLibrary.SphereTraceSingle` _pointinworldspace _pointinworldspace 10.0 "TraceTypeQuery1" false (`|MakeArray` self :!type "Actor Object Reference")))
  (if _returnvalue_2
    (return false (0.0 0.0 0.0))
    (elif _returnvalue
      (bind _output_get (set `local.Point` _projectedlocation))
      (return true (`self.FloorVector` (`KismetMathLibrary.InverseTransformLocation` (`self.GetTransform`) _output_get)))
      (else
        (return false (0.0 0.0 0.0))))))

(fn `CloserToPlayer b/w2`
  (params (Point1 :type "Vector Structure") (Point2 :type "Vector Structure"))
  (returns (ReturnValue :type Boolean))
  (bind _player_last_known_location (`self.Player Last Known Location`))
  (return (< (`KismetMathLibrary.Vector_DistanceSquared` (`local.Point1`) _player_last_known_location) (`KismetMathLibrary.Vector_DistanceSquared` _player_last_known_location (`local.Point2`)))))

(fn `CreateCoverPoints`
  (params (PeakPoint :type "Vector3f Structure"))
  (bind (_x _y _z) (`KismetMathLibrary.BreakVector3f` (`local.PeakPoint`)))
  (bind (_x_2 _y_2 _z_2) (`KismetMathLibrary.BreakVector3f` (`local.PeakPoint`)))
  (bind (_returnvalue_x _returnvalue_y) (`KismetMathLibrary.BreakVector` (`BoxComponent.GetUnscaledBoxExtent` (`self.CoverBox`))))
  (bind _returnvalue_x_2 (`KismetMathLibrary.BreakVector` (`BoxComponent.GetUnscaledBoxExtent` (`self.CoverBox`))))
  (if (>= (- _returnvalue_x_2 70.0) 100.0)
    (bind (_bvalidpoint _returnvalue) (`self.CheckForPointValidity` (`KismetMathLibrary.MakeVector` (+ (* (`self.temp`) (`KismetMathLibrary.SelectFloat` 1.0 -1.0 (> _x_2 0.0))) _x_2) _y_2 (+ _z_2 30.0))))
    (if _bvalidpoint
      (`KismetArrayLibrary.Array_Add` (`self.CoverPoints`) _returnvalue)))
  (if (>= (- _returnvalue_y 70.0) 100.0)
    (bind (_bvalidpoint_2 _returnvalue_2) (`self.CheckForPointValidity` (`KismetMathLibrary.MakeVector` _x (+ _y (* (`KismetMathLibrary.SelectFloat` 1.0 -1.0 (> _y 0.0)) (`self.temp`))) (+ _z 30.0))))
    (if _bvalidpoint_2
      (`KismetArrayLibrary.Array_Add` (`self.CoverPoints`) _returnvalue_2))))

(fn `CreatePoint`
  (returns (ReturnValue :type "Vector Structure"))
  (bind _coverpointscale (`self.CoverPointScale`))
  (bind (_x _y) (`KismetMathLibrary.BreakVector3f` (`BoxComponent.BoxExtent` (`self.CoverBox`))))
  (return (`KismetMathLibrary.MakeVector` (* _x (`self.X`) _coverpointscale) (* _y (`self.Y`) _coverpointscale))))

(fn `Farthese2Points`
  (params (Array :type "Array of Vector Structure") (DistanceFrom :type "Vector Structure") (`bFarthest?` :type Boolean))
  (returns (CoverPoint1 :type "Vector Structure") (CoverPoint2 :type "Vector Structure"))
  (locals (ArrayElem :type "Vector Structure") (Distance :type "Float (double-precision)") (CoverDistance2 :type "Float (double-precision)") (CoverDistance :type "Float (double-precision)") (LCoverLocation2 :type "Vector Structure") (LCoverLocation :type "Vector Structure"))
  (bind _coverdistance (`local.CoverDistance`))
  (bind _distance (`local.Distance`))
  (bind _coverdistance2 (`local.CoverDistance2`))
  (bind _coverdistance_2 (`local.CoverDistance`))
  (bind _distance_2 (`local.Distance`))
  (set `local.CoverDistance` (select `bool` `bFarthest?` :`false` 100000000.0))
  (for _array_element Array
    (bind _output_get (set `local.ArrayElem` _array_element))
    (set `local.Distance` (`KismetMathLibrary.Vector_DistanceSquared` _output_get (`local.DistanceFrom`)))
    (if (select `bool` (`local.bFarthest?`) :`false` (< _distance_2 _coverdistance) :`true` (> _distance_2 _coverdistance))
      (set `local.CoverDistance2` (`local.CoverDistance`))
      (set `local.LCoverLocation2` (`local.LCoverLocation`))
      (set `local.CoverDistance` (`local.Distance`))
      (set `local.LCoverLocation` (`local.ArrayElem`))
      (elif (select `bool` (`local.bFarthest?`) :`false` (and (< _distance _coverdistance2) (> _coverdistance2 _coverdistance_2)) :`true` (and (> _distance _coverdistance2) (< _coverdistance2 _coverdistance_2)))
        (set `local.CoverDistance2` (`local.Distance`))
        (set `local.LCoverLocation2` (`local.ArrayElem`)))))
  (return (`local.LCoverLocation`) (`local.LCoverLocation2`)))

(fn `FloorVector`
  (params (InVector :type "Vector Structure"))
  (returns (OutVector :type "Vector Structure"))
  (bind (_x _y _z) (`KismetMathLibrary.BreakVector3f` InVector))
  (return (`KismetMathLibrary.MakeVector` (`KismetMathLibrary.Conv_IntToDouble` (`KismetMathLibrary.FFloor` _x)) (`KismetMathLibrary.Conv_IntToDouble` (`KismetMathLibrary.FFloor` _y)) (`KismetMathLibrary.Conv_IntToDouble` (`KismetMathLibrary.FFloor` _z)))))

(fn `Give Peak Points`
  (params (CoverPointLocation :type "Vector Structure") (Array :type "Array of Vector Structure"))
  (returns (PeakPoint :type "Vector Structure"))
  (locals (PeakDistance1 :type "Float (double-precision)" :default 1000000.0) (PeakPoint1 :type "Vector Structure") (`PeakDistance 2` :type "Float (double-precision)" :default 1000000.0) (PeakPoint2 :type "Vector Structure") (ArrayElem :type "Vector Structure") (Distance :type "Float (double-precision)" :default 0.0))
  (bind _returnvalue (`KismetMathLibrary.Vector_Distance` (`local.ArrayElem`) (`local.CoverPointLocation`)))
  (for _array_element Array
    (set `local.ArrayElem` _array_element)
    (if (< _returnvalue (`local.PeakDistance1`))
      (set `local.PeakDistance1` _returnvalue)
      (set `local.PeakPoint1` (`local.ArrayElem`))))
  (return (`local.PeakPoint1`)))

(fn `GiveCoverPoint`
  (params (Array :type "Array of Vector Structure"))
  (returns (CoverLocation :type "Vector Structure"))
  (locals (CoverIndex :type Integer) (CoverDistance :type "Float (double-precision)" :default 0.0) (LCoverLocation :type "Vector Structure") (CoverDistance2 :type "Float (double-precision)") (LCoverLocation2 :type "Vector Structure") (ArrayElem :type "Vector Structure") (Distance :type "Float (double-precision)" :default 0.0))
  (if (> (`KismetArrayLibrary.Array_Length` Array) 1)
    (bind (_coverpoint1 _coverpoint2) (`self.Farthese2Points` (`local.Array`) (`self.Player Last Known Location`) true))
    (bind _finalcoverpoint (`self.SelectBestCrouchCoverPoint` _coverpoint1 _coverpoint2))
    (return _finalcoverpoint)
    (else
      (return (`|GetArrayItem` Array)))))

(fn `HitCountForCrouchCover`
  (params (CoverPoint :type "Vector Structure"))
  (returns (HitCount1 :type Integer))
  (locals (HitCount :type Integer))
  (for _array_element (`self.TestingArray`)
    (bind (_outhit _returnvalue) (`KismetSystemLibrary.LineTraceSingle` (+ (`local.CoverPoint`) _array_element) (+ (`self.Player Last Known Location`) (0.0 0.0 50.0)) "TraceTypeQuery1" false (`|MakeArray` (`GameplayStatics.GetPlayerPawn` 0) self (`self.GetOwner`) :!type "Actor Object Reference")))
    (if (not _returnvalue)
      (`/Engine/EditorBlueprintResources/StandardMacros.IncrementInt` (`local.HitCount`))))
  (return (`local.HitCount`)))

(fn `PeakCoverTesting`
  (returns (`Peak Point` :type "Vector Structure") (CoverPoint :type "Vector Structure"))
  (locals (LocalPeakPoints :type "Array of Vector Structure") (FarthestPeakPoint :type "Vector Structure") (Distance :type "Float (double-precision)" :default 0.0) (FinalPeakPoint :type "Vector Structure") (ClosestPeakPoint :type "Vector Structure")))

(fn `SelectBestCrouchCoverPoint`
  (params (CoverPoint1 :type "Vector Structure") (CoverPoint2 :type "Vector Structure"))
  (returns (FinalCoverPoint :type "Vector Structure"))
  (locals (HitCount1 :type Integer :default 0) (HitCount2 :type Integer :default 0) (FinalCover :type "Vector Structure"))
  (bind _hitcount1 (`self.HitCountForCrouchCover` CoverPoint1))
  (bind _output_get (set `local.HitCount1` _hitcount1))
  (bind _hitcount1_2 (`self.HitCountForCrouchCover` CoverPoint2))
  (set `local.HitCount2` _hitcount1_2)
  (`/Engine/EditorBlueprintResources/StandardMacros.CompareInt` (`local.HitCount1`) (`local.HitCount2`)
    (:`>`
      (set `local.FinalCover` (`local.CoverPoint1`) :!label _label))
    (:`==`
      (goto _label))
    (:`<`
      (set `local.FinalCover` (`local.CoverPoint2`))))
  (return (`local.FinalCover`)))

(fn `UserConstructionScript`
  (`PrimitiveComponent.SetMaterial` (`self.Cube`) 0 (select `bool` (`self.bIsStandingCover`) :`false` "/Game/Materials/MI_color2.MI_color2" :`true` "/Game/Materials/MI_color1.MI_color1" :!type "MaterialInterface Object Reference")))
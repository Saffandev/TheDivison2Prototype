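; AI cover actor that generates peek and cover points around its box and picks the best pair against the player.
; Generate_1 builds local corner points and offset cover spots, validated by sphere traces and navmesh projection; BeginPlay converts them to world space.
; BestCover chooses by stance: standing favours a side corner and its cover spot farther from the player; crouch compares the two farthest spots by unblocked traces to the player.
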(event `self.ReceiveBeginPlay`
  (set `self.NonTransformedPeak Points` (`self.PeakPoints`))
  (for (_array_element _array_index) (`self.PeakPoints`)
    (`KismetArrayLibrary.Array_Set` (`self.PeakPoints`) _array_index (`KismetMathLibrary.TransformLocation` (`self.GetTransform`) _array_element)))
  (for (_array_element_2 _array_index_2) (`self.CoverPoints`)
    (`KismetArrayLibrary.Array_Set` (`self.CoverPoints`) _array_index_2 (`KismetMathLibrary.TransformLocation` (`self.GetTransform`) _array_element_2))))

(event `Generate_1`
  (bind _points (`self.Points`))
  (bind (_returnvalue_x _returnvalue_y) (`KismetMathLibrary.BreakVector` (`BoxComponent.GetUnscaledBoxExtent` (`self.CoverBox`))))
  (`|ExecutionSequence`
    (:`then_0`
      (set `self.InitActorRotaion` (`self.K2_GetActorRotation`))
      (`KismetArrayLibrary.Array_Clear` (`self.PeakPoints`))
      (`KismetArrayLibrary.Array_Clear` (`self.CoverPoints`))
      (bind _index (`/Game/AI/AIMacro.ForLoopFloat` -1.0 1.0 (`self.CalculateLoopIncrement` _returnvalue_x))
        (:`LoopBody`
          (set `self.X` _index)
          (bind _index_2 (`/Game/AI/AIMacro.ForLoopFloat` -1.0 1.0 (`self.CalculateLoopIncrement` _returnvalue_y))
            (:`LoopBody`
              (set `self.Y` _index_2)
              (if (and (== (`self.X`) 0.0) (== (`self.Y`) 0.0))
                _
                (elif (== (+ (`KismetMathLibrary.Abs` (`self.X`)) (`KismetMathLibrary.Abs` (`self.Y`))) 2.0)
                  (bind (_bvalidpoint _returnvalue) (`self.CheckForPointValidity` (`self.CreatePoint`)))
                  (if _bvalidpoint
                    (set `self.Points` _returnvalue)
                    (`KismetArrayLibrary.Array_Add` (`self.PeakPoints`) _points)
                    (`self.CreateCoverPoints` _points)))))))))
    (:`then_1`
      (`SceneComponent.SetWorldScale3D` (`self.Cube`) (/ (`BoxComponent.BoxExtent` (`self.CoverBox`)) 100.0))
      (`CoverObject.SetNavModifierExtent` null (+ (/ (`BoxComponent.BoxExtent` (`self.CoverBox`)) 2.0) 60)))))

(event `CoverPointTesting`)

(fn `BestCover`
  (returns (CoverPoint :type "Vector Structure") (PeakPoint :type "Vector Structure"))
  (locals (Peak :type "Array of Vector Structure") (Cover :type "Array of Vector Structure") (TempCover :type "Vector Structure" :default (0.0 0.0 0.0)) (TempPeak :type "Vector Structure" :default (0.0 0.0 0.0)))
  (if (`self.bIsStandingCover`)
    (bind (_peak_point _coverpoint) (`self.PeakCoverTesting`))
    (return _coverpoint _peak_point)
    (else
      (set `local.Peak` (`self.PeakPoints`))
      (set `local.Cover` (`self.CoverPoints`))
      (bind _coverlocation (`self.GiveCoverPoint` (`local.Cover`)))
      (set `local.TempCover` _coverlocation)
      (bind _peakpoint (`self.Give Peak Points` (`local.TempCover`) (`local.Peak`)))
      (set `local.TempPeak` _peakpoint)
      (return (`local.TempCover`) (`local.TempPeak`)))))

(fn `BestCover_0`
  (returns (CoverPoint :type "Vector Structure") (PeakPoint :type "Vector Structure"))
  (locals (Peak :type "Array of Vector Structure") (Cover :type "Array of Vector Structure") (TempCover :type "Vector Structure" :default (0.0 0.0 0.0)) (TempPeak :type "Vector Structure" :default (0.0 0.0 0.0)))
  (set `local.Peak` (`self.PeakPoints`))
  (set `local.Cover` (`self.CoverPoints`))
  (bind _coverlocation (`self.GiveCoverPoint` (`local.Cover`) :!label _label))
  (set `local.TempCover` _coverlocation)
  (bind _peakpoint (`self.Give Peak Points` (`local.TempCover`) (`local.Peak`)))
  (set `local.TempPeak` _peakpoint)
  (if (`self.bIsStandingCover`)
    (if true
      _
      (elif (> (`KismetArrayLibrary.Array_Length` (`local.Cover`)) 1)
        (`KismetArrayLibrary.Array_RemoveItem` (`local.Cover`) (`local.TempCover`))
        (goto _label)
        (else
          _))))
  (return (`local.TempCover`) (`local.TempPeak`)))

(fn `CalculateLoopIncrement`
  (params (A :type "Float (double-precision)"))
  (returns (ReturnValue :type "Float (double-precision)"))
  (return (`KismetMathLibrary.FMax` (/ 1.0 (`KismetMathLibrary.Conv_IntToDouble` (`KismetMathLibrary.FFloor` (/ A 100.0)))) 0.5)))

(fn `CheckForPointValidity`
  (params (Point1 :type "Vector Structure"))
  (returns (bValidPoint :type Boolean) (ReturnValue :type "Vector Structure"))
  (locals (Point :type "Vector Structure") (PointInWorldSpace :type "Vector Structure" :default (0.0 0.0 0.0)))
  (bind _pointinworldspace (`local.PointInWorldSpace`))
  (bind (_projectedlocation _returnvalue) (`NavigationSystemV1.K2_ProjectPointToNavigation` (`local.PointInWorldSpace`) null "/Game/AI/Navigation/CoverNavFilter.CoverNavFilter_C" (50.0 50.0 200.0)))
  (set `local.Point` Point1)
  (set `local.PointInWorldSpace` (`KismetMathLibrary.TransformLocation` (`self.GetTransform`) (`local.Point`)))
  (bind (_outhit _returnvalue_2) (`KismetSystemLibrary.SphereTraceSingle` _pointinworldspace _pointinworldspace 10.0 "TraceTypeQuery1" false (`|MakeArray` self :!type "Actor Object Reference")))
  (if _returnvalue_2
    (return false (0.0 0.0 0.0))
    (elif _returnvalue
      (bind _output_get (set `local.Point` _projectedlocation))
      (return true (`KismetMathLibrary.InverseTransformLocation` (`self.GetTransform`) _output_get))
      (else
        (return false (0.0 0.0 0.0))))))

(fn `CreateCoverPoints`
  (params (PeakPoint :type "Vector3f Structure"))
  (bind (_x _y _z) (`KismetMathLibrary.BreakVector3f` (`local.PeakPoint`)))
  (bind (_x_2 _y_2 _z_2) (`KismetMathLibrary.BreakVector3f` (`local.PeakPoint`)))
  (bind (_bvalidpoint _returnvalue) (`self.CheckForPointValidity` (`KismetMathLibrary.MakeVector` (+ (* (`self.temp`) (`KismetMathLibrary.SelectFloat` 1.0 -1.0 (> _x_2 0.0))) _x_2) _y_2 (+ _z_2 30.0))))
  (if _bvalidpoint
    (`KismetArrayLibrary.Array_Add` (`self.CoverPoints`) _returnvalue))
  (bind (_bvalidpoint_2 _returnvalue_2) (`self.CheckForPointValidity` (`KismetMathLibrary.MakeVector` _x (+ _y (* (`KismetMathLibrary.SelectFloat` 1.0 -1.0 (> _y 0.0)) (`self.temp`))) (+ _z 30.0))))
  (if _bvalidpoint_2
    (`KismetArrayLibrary.Array_Add` (`self.CoverPoints`) _returnvalue_2)))

(fn `CreatePoint`
  (returns (ReturnValue :type "Vector Structure"))
  (bind _coverpointscale (`self.CoverPointScale`))
  (bind (_x _y) (`KismetMathLibrary.BreakVector3f` (`BoxComponent.BoxExtent` (`self.CoverBox`))))
  (return (+ (`KismetMathLibrary.MakeVector` (* _x (`self.X`) 1.0 _coverpointscale) (* _y (`self.Y`) 1.0 _coverpointscale)) (0.0 0.0 0.0))))

(fn `Farthese2Points`
  (params (Array :type "Array of Vector Structure") (DistanceFrom :type "Vector Structure") (`bFarthest?` :type Boolean))
  (returns (CoverPoint1 :type "Vector Structure") (CoverPoint2 :type "Vector Structure"))
  (locals (ArrayElem :type "Vector Structure") (Distance :type "Float (double-precision)") (CoverDistance2 :type "Float (double-precision)") (CoverDistance :type "Float (double-precision)") (LCoverLocation2 :type "Vector Structure") (LCoverLocation :type "Vector Structure"))
  (bind _coverdistance (`local.CoverDistance`))
  (bind _distance (`local.Distance`))
  (bind _coverdistance2 (`local.CoverDistance2`))
  (bind _coverdistance_2 (`local.CoverDistance`))
  (bind _distance_2 (`local.Distance`))
  (set `local.CoverDistance` (select `bool` `bFarthest?` :`false` 1000000.0))
  (for _array_element Array
    (bind _output_get (set `local.ArrayElem` _array_element))
    (set `local.Distance` (`KismetMathLibrary.Vector_DistanceSquared` _output_get DistanceFrom))
    (if (select `bool` (`local.bFarthest?`) :`false` (< _distance_2 _coverdistance) :`true` (> _distance_2 _coverdistance))
      (set `local.CoverDistance2` (`local.CoverDistance`))
      (set `local.LCoverLocation2` (`local.LCoverLocation`))
      (set `local.CoverDistance` (`local.Distance`))
      (set `local.LCoverLocation` (`local.ArrayElem`))
      (elif (select `bool` (`local.bFarthest?`) :`false` (and (< _distance _coverdistance2) (> _coverdistance2 _coverdistance_2)) :`true` (and (> _distance _coverdistance2) (< _coverdistance2 _coverdistance_2)))
        (set `local.CoverDistance2` (`local.Distance`))
        (set `local.LCoverLocation2` (`local.ArrayElem`)))))
  (return (`local.LCoverLocation`) (`local.LCoverLocation2`)))

(fn `Give Peak Points`
  (params (CoverPointLocation :type "Vector Structure") (Array :type "Array of Vector Structure"))
  (returns (PeakPoint :type "Vector Structure"))
  (locals (PeakDistance1 :type "Float (double-precision)" :default 1000000.0) (PeakPoint1 :type "Vector Structure") (`PeakDistance 2` :type "Float (double-precision)" :default 1000000.0) (PeakPoint2 :type "Vector Structure") (ArrayElem :type "Vector Structure") (Distance :type "Float (double-precision)" :default 0.0))
  (bind _returnvalue (`KismetMathLibrary.Vector_Distance` (`local.ArrayElem`) (`local.CoverPointLocation`)))
  (for _array_element Array
    (set `local.ArrayElem` _array_element)
    (if (< _returnvalue (`local.PeakDistance1`))
      (set `local.PeakDistance1` _returnvalue)
      (set `local.PeakPoint1` (`local.ArrayElem`))))
  (return (`local.PeakPoint1`)))

(fn `GiveCoverPoint`
  (params (Array :type "Array of Vector Structure"))
  (returns (CoverLocation :type "Vector Structure"))
  (locals (CoverIndex :type Integer) (CoverDistance :type "Float (double-precision)" :default 0.0) (LCoverLocation :type "Vector Structure") (CoverDistance2 :type "Float (double-precision)") (LCoverLocation2 :type "Vector Structure") (ArrayElem :type "Vector Structure") (Distance :type "Float (double-precision)" :default 0.0))
  (if (> (`KismetArrayLibrary.Array_Length` Array) 1)
    (bind (_coverpoint1 _coverpoint2) (`self.Farthese2Points` (`local.Array`) (`self.K2_GetActorLocation` (`GameplayStatics.GetPlayerPawn` 0)) true))
    (bind _finalcoverpoint (`self.SelectBestCrouchCoverPoint` _coverpoint1 _coverpoint2))
    (return _finalcoverpoint)
    (else
      (return (`|GetArrayItem` Array)))))

(fn `HitCountForCrouchCover`
  (params (CoverPoint :type "Vector Structure"))
  (returns (HitCount1 :type Integer))
  (locals (HitCount :type Integer))
  (bind _returnvalue (`GameplayStatics.GetPlayerPawn` 0))
  (for _array_element (`self.TestingArray`)
    (bind (_outhit _returnvalue_2) (`KismetSystemLibrary.LineTraceSingle` (+ (`local.CoverPoint`) _array_element) (+ (`self.K2_GetActorLocation` _returnvalue) (0.0 0.0 50.0)) "TraceTypeQuery1" false (`|MakeArray` _returnvalue self :!type "Actor Object Reference") "ForOneFrame"))
    (if (not _returnvalue_2)
      (`/Engine/EditorBlueprintResources/StandardMacros.IncrementInt` (`local.HitCount`))))
  (return (`local.HitCount`)))

(fn `PeakCoverTesting`
  (returns (`Peak Point` :type "Vector Structure") (CoverPoint :type "Vector Structure"))
  (locals (LocalPeakPoints :type "Array of Vector Structure") (NewLocalVar :type "Vector Structure") (Distance :type "Float (double-precision)" :default 0.0) (FinalPeakPoint :type "Vector Structure") (farthestPeakPoing :type "Vector Structure"))
  (bind (_farthestpeakpoing_x _farthestpeakpoing_y _farthestpeakpoing_z) (`KismetMathLibrary.BreakVector` (`local.farthestPeakPoing`)))
  (bind _peakpoint (`self.Give Peak Points` (`self.K2_GetActorLocation` (`GameplayStatics.GetPlayerPawn` 0)) (`self.PeakPoints`)))
  (set `local.farthestPeakPoing` _peakpoint)
  (if (> (`KismetArrayLibrary.Array_Length` (`self.PeakPoints`)) 2)
    (set `local.LocalPeakPoints` (`self.PeakPoints`))
    (`KismetArrayLibrary.Array_RemoveItem` (`local.LocalPeakPoints`) (`local.farthestPeakPoing`))
    (set `local.farthestPeakPoing` (`KismetMathLibrary.InverseTransformLocation` (`self.GetTransform`) (`local.farthestPeakPoing`)))
    (bind _output_get (set `local.NewLocalVar` (`KismetMathLibrary.MakeVector` (* _farthestpeakpoing_x -1.0) (* _farthestpeakpoing_y -1.0) _farthestpeakpoing_z)))
    (set `local.NewLocalVar` (`KismetMathLibrary.TransformLocation` (`self.GetTransform`) _output_get))
    (`KismetArrayLibrary.Array_RemoveItem` (`local.LocalPeakPoints`) (`local.NewLocalVar`))
    (for _array_element (`local.LocalPeakPoints`)
      (bind _returnvalue (`KismetMathLibrary.Vector_Distance` _array_element (`self.K2_GetActorLocation` (`GameplayStatics.GetPlayerPawn` 0))))
      (if (> _returnvalue (`local.Distance`))
        (set `local.FinalPeakPoint` _array_element)
        (set `local.Distance` _returnvalue)))
    (else
      (set `local.FinalPeakPoint` (`local.farthestPeakPoing`))))
  (bind (_coverpoint1 _coverpoint2) (`self.Farthese2Points` (`self.CoverPoints`) (`local.FinalPeakPoint`)))
  (return (`local.FinalPeakPoint`) (select `bool` (`self.WhichIsSmaller` _coverpoint1 _coverpoint2) :`false` _coverpoint1 :`true` _coverpoint2)))

(fn `SelectBestCrouchCoverPoint`
  (params (CoverPoint1 :type "Vector Structure") (CoverPoint2 :type "Vector Structure"))
  (returns (FinalCoverPoint :type "Vector Structure"))
  (locals (HitCount1 :type Integer :default 0) (HitCount2 :type Integer :default 0) (FinalCover :type "Vector Structure"))
  (bind _hitcount1 (`self.HitCountForCrouchCover` CoverPoint1))
  (set `local.HitCount1` _hitcount1)
  (bind _hitcount1_2 (`self.HitCountForCrouchCover` CoverPoint2))
  (set `local.HitCount2` _hitcount1_2)
  (`/Engine/EditorBlueprintResources/StandardMacros.CompareInt` (`local.HitCount1`) (`local.HitCount2`)
    (:`>`
      (set `local.FinalCover` (`local.CoverPoint1`)))
    (:`==`
      (set `local.FinalCover` (`local.CoverPoint1`)))
    (:`<`
      (set `local.FinalCover` (`local.CoverPoint2`))))
  (return (`local.FinalCover`)))

(fn `UserConstructionScript`)

(fn `WhichIsSmaller`
  (params (Point1 :type "Vector Structure") (Point2 :type "Vector Structure"))
  (returns (ReturnValue :type Boolean))
  (bind _returnvalue (`self.K2_GetActorLocation` (`GameplayStatics.GetPlayerPawn` 0)))
  (return (< (`KismetMathLibrary.Vector_DistanceSquared` (`local.Point1`) _returnvalue) (`KismetMathLibrary.Vector_DistanceSquared` _returnvalue (`local.Point2`)))))
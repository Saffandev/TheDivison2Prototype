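; AI combat character whose type selects a traits data asset for health, weapon and stun tuning, plus a body material.
; On spawn it attaches its gun, then exposes timed firing and montage-led grenade throws using suggested projectile velocity.
; Damage feeds a timed stun meter gated by StunCondition, whose check logic is unwired, and toggles blackboard cover availability to force re-evaluation.
; Combat state changes are mirrored to the AI controller's blackboard.
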(event `self.ReceiveBeginPlay`
  (bind (_aitraits_aitype _aitraits_bcantakecover _aitraits_bcanthrowgrenade _aitraits_walkingspeed _aitraits_sprintspeed _aitraits_adsspeed _aitraits_health _aitraits_advancingtime _aitraits_stunthreshold _aitraits_stunduration _aitraits_fireduration _aitraits_maxcombatrange _aitraits_mincombatrange _aitraits_gunclass) (break `AITraits` (`self.AITraits`)))
  (bind (_aitraits_aitype_2 _aitraits_bcantakecover_2 _aitraits_bcanthrowgrenade_2 _aitraits_walkingspeed_2 _aitraits_sprintspeed_2 _aitraits_adsspeed_2 _aitraits_health_2) (break `AITraits` (`self.AITraits`)))
  (bind (_value _returnvalue) (`BlueprintMapLibrary.Map_Find` (`self.AITypeData`) (`self.AIType`)))
  ;[1 1 1] Begin Play
  (bind _asbp_aicontroller (cast `/Game/AI/BP_AIController` (`AIBlueprintHelperLibrary.GetAIController` self)))
  (set `self.As BP AIController` _asbp_aicontroller)
  (if _returnvalue
    (set `self.AITraitsDataAsset` _value)
    (set `self.AITraits` (`AITraitsDataAsset.AITraits` (`self.AITraitsDataAsset`)))
    (bind _output_get (set `self.Health` _aitraits_health_2))
    (set `self.CurrentHealth` _output_get)
    ;[1 1 1] Giving Weapon
    (if (`KismetSystemLibrary.IsValidClass` _aitraits_gunclass)
      (bind _returnvalue_2 (`|SpawnActorFromClass` _aitraits_gunclass (`KismetMathLibrary.MakeTransform` (0.0 0.0 0.0)) "Undefined" "MultiplyWithRoot" self null))
      (bind _asbp_gun_base (cast `/Game/AI/Weapons/BP_GunBase` _returnvalue_2))
      (bind _output_get_2 (set `self.Gun_0` _asbp_gun_base))
      (`self.K2_AttachToComponent` _output_get_2 (`self.Mesh`) "Weapon" "SnapToTarget" "SnapToTarget" "KeepRelative" true)
      (else
        (`KismetSystemLibrary.PrintString` "No Weapon Class")))))

(event `StartFire`
  (bind (_aitraits_aitype _aitraits_bcantakecover _aitraits_bcanthrowgrenade _aitraits_walkingspeed _aitraits_sprintspeed _aitraits_adsspeed _aitraits_health _aitraits_advancingtime _aitraits_stunthreshold _aitraits_stunduration _aitraits_fireduration) (break `AITraits` (`self.AITraits`)))
  ;[1 1 1] Fire thing
  (`/Game/AI/Weapons/BP_GunBase.StartFire` (`self.Gun_0`) _aitraits_fireduration)
  (set `self.bIsFiring` true))

(event `StopFire`
  ;[1 1 1] Fire thing
  (`/Game/AI/Weapons/BP_GunBase.StopFire` (`self.Gun_0`))
  (set `self.bIsFiring` false))

(event `ThrowGrenade`
  (bind _returnvalue (`SceneComponent.GetSocketLocation` (`self.Mesh`) "hand_l"))
  ;[1 1 1] Grenade impact point calculation
  (bind (_tossvelocity _returnvalue_2) (`GameplayStatics.BlueprintSuggestProjectileVelocity` _returnvalue (`self.End Toss Loc`) 2000.0 0.0 "DoNotTrace" 5.0 false true))
  (if _returnvalue_2
    (`|SpawnActorFromClass` "/Game/Blueprints/BP_Grenade.BP_Grenade_C" (`KismetMathLibrary.MakeTransform` _returnvalue (struct) (0.1 0.1 0.1)) "Undefined" "MultiplyWithRoot" null _tossvelocity null)
    (`KismetSystemLibrary.Delay` 0.7)
    (`self.SetCombatState` "NewEnumerator3")))

(event `self.TookDamage`
  (params (DamageValue :type "Float (double-precision)"))
  (bind (_aitraits_aitype _aitraits_bcantakecover _aitraits_bcanthrowgrenade _aitraits_walkingspeed _aitraits_sprintspeed _aitraits_adsspeed _aitraits_health _aitraits_advancingtime _aitraits_stunthreshold _aitraits_stunduration) (break `AITraits` (`self.AITraits`)))
  (bind (_aitraits_aitype_2 _aitraits_bcantakecover_2 _aitraits_bcanthrowgrenade_2 _aitraits_walkingspeed_2 _aitraits_sprintspeed_2 _aitraits_adsspeed_2 _aitraits_health_2 _aitraits_advancingtime_2 _aitraits_stunthreshold_2) (break `AITraits` (`self.AITraits`)))
  (bind _returnvalue (`AIBlueprintHelperLibrary.GetBlackboard` (`self.As BP AIController`)))
  ;[1 1 1] Stun
  (`|ExecutionSequence`
    (:`then_0`
      (if (and (not (`BlackboardComponent.GetValueAsBool` (`AIBlueprintHelperLibrary.GetBlackboard` (`self.As BP AIController`)) "bStun")) (`self.bCanStunAgain`) (`self.bIsFiring`))
        (set `self.StunMeter` (+ DamageValue (`self.StunMeter`)))
        (bind _returnvalue_2 (`KismetSystemLibrary.K2_SetTimerDelegate` (`|CreateDelegate` :!event `ResetStun`) _aitraits_stunduration)) ; if the AI doesn't gets damage for 2 seconds, and stun meter will reset
        (set `self.StunTimer` _returnvalue_2)
        (if (> (`self.StunMeter`) _aitraits_stunthreshold_2)
          (`self.SetCombatState` "NewEnumerator2")
          (`|PlayMontage` (`self.Mesh`) "/Game/AnimStarterPack/Hit_React_1_Montage.Hit_React_1_Montage"
            (:`OnCompleted`
              (set `self.bCanStunAgain` false))))))
    (:`then_1`
      ;[1 1 1] cover re-eval on getting hit
      (if (`BlackboardComponent.GetValueAsBool` (`AIBlueprintHelperLibrary.GetBlackboard` (`self.As BP AIController`)) "bInCover")
        (`BlackboardComponent.SetValueAsBool` _returnvalue "bCoverAvailable" false)
        (`BlackboardComponent.SetValueAsBool` _returnvalue "bCoverAvailable" true)))))

(event `initGrenadeThrow`
  (params (EndTossLoc :type "Vector Structure"))
  ;[1 1 1] throwing Grenade
  (set `self.End Toss Loc` EndTossLoc)
  (`self.PlayAnimMontage` "/Game/AnimStarterPack/Montage/MM_Rifle_GrenadeToss_Montage.MM_Rifle_GrenadeToss_Montage")
  (`self.SetCombatState` "NewEnumerator1"))

(event `ResetStun`
  ;[1 1 1] Stun
  (`KismetSystemLibrary.K2_ClearAndInvalidateTimerHandle` (`self.StunTimer`))
  (`self.SetCombatState` "NewEnumerator3")
  (set `self.StunMeter` 0.0)
  ;;[1 1 1] stun cooldown
  (`KismetSystemLibrary.Delay` 5.0)
  (set `self.bCanStunAgain` true))

(fn `Death`
  (`parent.Death`)
  (`self.K2_DestroyActor` (`self.Gun_0`)))

(fn `SetCombatState`
  (params (CombatState :type "/Game/AI/Enum/ECombatState Enum" :default "NewEnumerator0"))
  (bind _output_get (set `self.CombatState` CombatState))
  (`BlackboardComponent.SetValueAsEnum` (`/Game/AI/BP_AIController.MyBlackboard` (`self.As BP AIController`)) "CombatState" _output_get))

(fn `UserConstructionScript`
  (`PrimitiveComponent.SetMaterial` (`self.Mesh`) 0 (select `EAIType` (`self.AIType`) :`Rushers` "/Game/AnimStarterPack/UE4_Mannequin/Materials/MI_Manne_Rushers.MI_Manne_Rushers" :`Rangers` "/Game/AnimStarterPack/UE4_Mannequin/Materials/MI_Manne_Assault.MI_Manne_Assault" :`Shotgunner` "/Game/AnimStarterPack/UE4_Mannequin/Materials/MI_Manne_Shotgunner.MI_Manne_Shotgunner" :`HeavyMachineGunner` "/Game/AnimStarterPack/UE4_Mannequin/Materials/MI_Manne_LMG.MI_Manne_LMG" :!type "MaterialInterface Object Reference")))